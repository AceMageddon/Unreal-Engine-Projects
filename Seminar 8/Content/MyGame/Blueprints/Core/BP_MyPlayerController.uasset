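; Player controller for a platform game that creates the HUD and drives the possessed BP_Platform pawn.
; On BeginPlay it switches to game-only input and adds BP_HUD to the viewport.
; On possession it caches the platform, then the Left_Right axis slides it along Y with swept, frame-rate-independent movement.
; The SpawnBall action tells the platform to spawn a ball.
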(event EventBeginPlay
  (Input|SetInputModeGameOnly self false)
  (bind _returnvalue (UserInterface|CreateWidget "/Game/MyGame/Blueprints/BP_HUD.BP_HUD_C" self))
  (UserInterface|Viewport|AddtoViewport _returnvalue 0)
  (Variables|Default|SetHUD _returnvalue))

(event EventPossess
  (params (PossessedPawn :type Pawn%20Object%20Reference))
  (bind _asbp_platform (Utilities|Casting|CastToBP_Platform PossessedPawn))
  (Variables|Default|SetMyPawn _asbp_platform))

(event Input|ActionEvents|InputActionSpawnBall
  (params (Key :type Key%20Structure :default "None"))
  (:Pressed
    (Default|SpawnBall (Variables|Default|GetMyPawn))))

(event Input|AxisEvents|InputAxisLeft_Right
  (params (AxisValue :type Float%20%28single-precision%29))
  (Transformation|AddActorWorldOffset (Variables|Default|GetMyPawn) (Math|Vector|MakeVector 0.0 (* AxisValue (Utilities|Time|GetWorldDeltaSeconds) (Variables|Default|GetSpeed)) 0.0) true))

(fn ConstructionScript)