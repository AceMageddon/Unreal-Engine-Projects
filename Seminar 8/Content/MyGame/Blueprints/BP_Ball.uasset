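; BP_Ball is a ball actor that bounces off whatever blocks it and gets faster with each hit.
; Tick moves it by Speed, Direction and delta time in a swept world offset, using only the X and Y components.
; On a blocking hit, it reflects Direction about the hit normal and adds AddSpeed to Speed, with no upper limit.
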(event EventBeginPlay)

(event Collision|EventActorBeginOverlap
  (params (OtherActor :type Actor%20Object%20Reference)))

(event EventTick
  (params (DeltaSeconds :type Float%20%28single-precision%29))
  ;[1 1 1] Логика движения шара
  (bind _sweephitresult (Transformation|AddActorWorldOffset (Math|Vector|MakeVector (.x (* (* (Variables|Default|GetSpeed) (Variables|Default|GetDirection)) DeltaSeconds)) (.y (* (* (Variables|Default|GetSpeed) (Variables|Default|GetDirection)) DeltaSeconds)) 0.0) true))
  (if (.bBlockingHit (Collision|BreakHitResult _sweephitresult))
    (Variables|Default|SetDirection (Math|Vector|GetReflectionVector (Variables|Default|GetDirection) (.Normal (Collision|BreakHitResult _sweephitresult))))
    ;[1 1 1] Увеличение скорости шара при столкновении
    (Variables|Default|SetSpeed (+ (Variables|Default|GetSpeed) (Variables|Default|GetAddSpeed)))))

(fn ConstructionScript)