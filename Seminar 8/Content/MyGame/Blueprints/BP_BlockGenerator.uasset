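; Grid generator actor that lays out the level's field of BP_Block_Child blocks from X, Y and Padding settings.
; The Construction Script builds a static mesh preview grid for the viewport.
; BeginPlay destroys the preview and spawns the blocks in a grid at the actor's location, spaced at twice Padding, unlike the preview.
; Spawned blocks are stored in an array, whose length GetCubesForWin returns as the win count.
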(event EventBeginPlay
  (bind _returnvalue (Transformation|GetActorLocation))
  ;[1 1 1] Уничтожение сгенерированных кубов (эти нужны только для отображения сетки во Viewport)
  (for _array_element (Variables|Default|GetCubePreviewArray)
    (Components|DestroyComponent _array_element))
  ;[1 1 1] Генерация BP_Block_Child в сетку Vieport
  (for _index (range 0 (Variables|Default|GetX))
    (for _index_2 (range 0 (Variables|Default|GetY))
      (bind _returnvalue_2 (Game|SpawnActorfromClass "/Game/MyGame/Blueprints/BP_Block_Child.BP_Block_Child_C" (Math|Transform|MakeTransform (Math|Vector|MakeVector (+ (.x _returnvalue) (Math|Conversions|ToFloat(Integer) (* _index (* (Variables|Default|GetPadding) 2)))) (+ (.y _returnvalue) (Math|Conversions|ToFloat(Integer) (* _index_2 (* (Variables|Default|GetPadding) 2)))) (.z _returnvalue))) "Undefined" "MultiplyWithRoot" 0 0))
      ;[1 1 1] Сколько кубов на поле
      (Utilities|Array|Add (Variables|Default|GetCubesOnFieldArray) _returnvalue_2))))

(fn ConstructionScript
  ;[1 1 1] Генерация сетки кубов
  (for _index (range 0 (Variables|Default|GetX))
    (for _index_2 (range 0 (Variables|Default|GetY))
      (bind _returnvalue (AddComponent|AddStaticMeshComponent false (Math|Transform|MakeTransform (Math|Vector|MakeVector (Math|Conversions|ToFloat(Integer) (* _index (Variables|Default|GetPadding))) (Math|Conversions|ToFloat(Integer) (* _index_2 (Variables|Default|GetPadding))) 0.0))))
      (Utilities|Array|Add (Variables|Default|GetCubePreviewArray) _returnvalue))))

(fn GetCubesforWin
  (return (Utilities|Array|Length (Variables|Default|GetCubesOnFieldArray))))