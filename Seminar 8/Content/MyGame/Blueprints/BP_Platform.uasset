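; BP_Platform is the player's platform in a ball game, handling ball spawning, lives and bonus pickups.
; SpawnBall spawns a ball at the Arrow if lives remain and none is tracked; its destruction costs a life.
; Cube overlaps with BP_Bonuses widen the platform once, add a life or spawn an extra, untracked ball.
; Life changes fire the LivesChanged dispatcher, and losing the last life prints game over.
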(event OnComponentBeginOverlap(Cube)
  (params (OverlappedComponent :type Primitive%20Component%20Object%20Reference) (OtherActor :type Actor%20Object%20Reference) (OtherComp :type Primitive%20Component%20Object%20Reference) (OtherBodyIndex :type Integer) (bFromSweep :type Boolean) (SweepResult :type Hit%20Result%20Structure%20%28by%20ref%29))
  ;[1 1 1] Применение бонуса
  (bind _asbp_bonuses (Utilities|Casting|CastToBP_Bonuses OtherActor))
  (switch Utilities|FlowControl|Switch|SwitchonE_BonusType (Variables|/Game/MyGame/Blueprints/Bonuses/BP_Bonuses.BP_Bonuses_C|GetBonusType _asbp_bonuses)
    (:NewEnumerator0
      (CallFunction|MaximizeFlatformEvent))
    (:NewEnumerator1
      (CallFunction|AddLiveEvent))
    (:NewEnumerator2
      (CallFunction|AddBallEvent)))
  (Actor|DestroyActor _asbp_bonuses))

(event Custom|SpawnBall
  ;[1 1 1] Спаун шара только при условии того, что он не валиден (уничтожен килл-зоной)
  (if (not (<= (Variables|Default|GetPlayerLives) 0))
    (Variables|Default|GetBallIsAlive
      (:then)
      (:else
        (bind _returnvalue (Game|SpawnActorfromClass "/Game/MyGame/Blueprints/BP_Ball.BP_Ball_C" (Math|Transform|MakeTransform (Transformation|GetWorldLocation (Variables|Default|GetArrow))) "Undefined" "MultiplyWithRoot" 0 0))
        (bind _output_get (Variables|Default|SetBallIsAlive _returnvalue))
        ;[1 1 1] Конец игры, если жизни Игрока закончились
        (Game|BindEventtoOnDestroyed _output_get (delegate Custom|PlayerDead))))))

(event Custom|PlayerDead
  (params (DestroyedActor :type Actor%20Object%20Reference))
  ;[1 1 1] Конец игры, если жизни Игрока закончились
  (bind _result (Math|Integer|DecrementInt (Variables|Default|GetPlayerLives))
    (:%20%20
      (Default|CallLivesChanged _result)
      (if (<= _result 0)
        (Development|PrintText "GAME OVER!!!")))))

(event Custom|MaximizeFlatform%20Event
  (bind _cube (Variables|Default|GetCube))
  (bind _relativescale3d (Variables|/Script/Engine.SceneComponent|GetRelativeScale3D _cube))
  ;[1 1 1] Бонус: увеличение размера платформы
  (if (not (Variables|Default|GetisPlatformMaximized))
    (Transformation|SetRelativeScale3D _cube (Math|Vector|MakeVector (.x _relativescale3d) (* (.y _relativescale3d) 1.5) (.z _relativescale3d)))
    (Variables|Default|SetisPlatformMaximized true)))

(event Custom|AddLive%20Event
  ;[1 1 1] Бонус: увеличение жизней Игрока
  (bind _result (Math|Integer|IncrementInt (Variables|Default|GetPlayerLives))
    (:%20%20
      ;[1 1 1] Вызов dispatcher, который будет отображать кол-во жизней
      (Default|CallLivesChanged _result))))

(event Custom|AddBall%20Event
  ;[1 1 1] Бонус: добавление ещё одного шара
  (bind _returnvalue (Game|SpawnActorfromClass "/Game/MyGame/Blueprints/BP_Ball.BP_Ball_C" (Math|Transform|MakeTransform (Transformation|GetWorldLocation (Variables|Default|GetArrow))) "Undefined" "MultiplyWithRoot" 0 0))
  (Rendering|Material|SetMaterial (Variables|/Game/MyGame/Blueprints/BP_Ball.BP_Ball_C|GetSphere _returnvalue) 0 "/Engine/MapTemplates/Materials/BasicAsset03.BasicAsset03"))

(fn ConstructionScript)