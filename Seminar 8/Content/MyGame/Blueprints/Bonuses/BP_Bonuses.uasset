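; BP_Bonuses is a moving bonus Actor with a randomly assigned type.
; The Construction Script picks one of three BonusType enum values at random and shows its name on a TextRender component.
; Each Tick moves the Actor with a swept world offset along X only, using the X component of Speed, Direction and delta time multiplied together.
; It contains no active overlap or pickup logic.
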(event EventBeginPlay)

(event Collision|EventActorBeginOverlap
  (params (OtherActor :type Actor%20Object%20Reference)))

(event EventTick
  (params (DeltaSeconds :type Float%20%28single-precision%29))
  ;[1 1 1] Генерация бонусов
  (Transformation|AddActorWorldOffset (Math|Vector|MakeVector (.x (* (* (Variables|Default|GetSpeed) DeltaSeconds) (Variables|Default|GetDirection))) 0.0 0.0) true))

(fn ConstructionScript
  ;[1 1 1] Рандомизация бонусов
  (Variables|Default|SetBonusType (Utilities|Select :Index (Math|Random|RandomIntegerinRange 0 2) :Option%200 "NewEnumerator0" :Option%201 "NewEnumerator1" :Option%202 "NewEnumerator2"))
  (Rendering|Components|TextRender|SetText (Variables|Default|GetTextRender) (Utilities|Text|ToText(String) (Utilities|String|EnumtoString (Variables|Default|GetBonusType)))))